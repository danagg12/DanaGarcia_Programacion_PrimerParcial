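; BP_Enemigo is an enemy actor that moves by a local velocity offset and can fire BP_Bala projectiles.
; Tick applies VelocidadEnemigos every frame without sweep or delta-time scaling.
; SpawnBala spawns a bullet at the enemy's location, passing it VelocidadBala.
; Setter functions replace the movement velocity and multiply the current bullet velocity vector by a scalar, so repeated calls compound.
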(event EventTick
  (params (DeltaSeconds :type Float%20%28single-precision%29))
  (Transformation|AddActorLocalOffset (Variables|Default|GetVelocidad%20Enemigos) false false))

(fn ConstructionScript)

(fn SpawnBala
  (Game|SpawnActorfromClass "/Game/BluePrint/BP_Bala.BP_Bala_C" (Math|Transform|MakeTransform (Transformation|GetActorLocation) "0, 0, 0" "1.000000,1.000000,1.000000") "Undefined" "MultiplyWithRoot" 0 (Variables|Default|GetVelocidad%20Bala) 0))

(fn VelocidadEnemigo
  (params (Velocidad :type Vector))
  (Variables|Default|SetVelocidad%20Enemigos Velocidad))

(fn VelocidadBala
  (params (Velocidad :type Float%20%28double-precision%29) (VelocidadBala :type Vector))
  (bind _output_get (Variables|Default|SetVelocidadBala2 Velocidad))
  (Variables|Default|SetVelocidad%20Bala (Math|Vector|MakeVector (* _output_get (.x VelocidadBala)) (* _output_get (.y VelocidadBala)) (* _output_get (.z VelocidadBala)))))